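; Moving platform Blueprint that travels between two points and periodically rotates, as a flipping platform.
; The construction script adds Location01 and Location02 as relative control points on an InterpToMovement component, which handles the travel.
; From BeginPlay, an endless delay loop waits SecondsBetweenRotation, activates RotatingMovement for SecondsToRotate, then deactivates it, independently of the linear movement.
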(event `self.ReceiveBeginPlay`
  (`KismetSystemLibrary.Delay` (`self.Seconds Between Rotation`) :!label _label)
  (`ActorComponent.Activate` (`self.RotatingMovement`) false)
  (`KismetSystemLibrary.Delay` (`self.Seconds To Rotate`))
  (`ActorComponent.Deactivate` (`self.RotatingMovement`))
  (goto _label))

(fn `UserConstructionScript`
  (`InterpToMovementComponent.AddControlPointPosition` (`self.InterpToMovement`) (`self.Location01`) true)
  (`InterpToMovementComponent.AddControlPointPosition` (`self.InterpToMovement`) (`self.Location02`) true))